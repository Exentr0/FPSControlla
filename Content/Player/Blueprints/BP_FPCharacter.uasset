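; First-person player character Blueprint that drives head-bob camera shakes from the character's movement state.
; Each Tick calls HeadBob, which casts the StateManager's current state to FPCharacterGroundedState and does nothing if that fails.
; The state's display name selects an idle, walking or light-landing shake, started on player controller 0 every frame while that state holds.
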(event Custom|HeadBob
  (bind _returnvalue (Game|GetPlayerController 0))
  ;[1 1 1] Camera Shake
  (bind _asfpcharacter_grounded_state (Utilities|Casting|CastToFPCharacterGroundedState (Variables|/Script/CustomStateMachine.StateManagerComponent|GetCurrentState (Variables|Default|GetStateManager))))
  (switch string (Utilities|String|ToString(Name) (Variables|/Script/CustomStateMachine.BaseState|GetStateDisplayName _asfpcharacter_grounded_state))
    (:Idle
      (Game|Feedback|ClientStartCameraShake _returnvalue "/Game/Player/Blueprints/Headbob/Idle.Idle_C" 1.0 "CameraLocal" "0, 0, 0"))
    (:Walking
      (Game|Feedback|ClientStartCameraShake _returnvalue "/Game/Player/Blueprints/Headbob/Walk.Walk_C" 1.0 "CameraLocal" "0, 0, 0"))
    (:LightLanding
      (Game|Feedback|ClientStartCameraShake _returnvalue "/Game/Player/Blueprints/Headbob/LightLanding.LightLanding_C" 1.0 "CameraLocal" "0, 0, 0"))))

(event EventTick
  (params (DeltaSeconds :type Float%20%28single-precision%29))
  (CallFunction|HeadBob))

(fn ConstructionScript)